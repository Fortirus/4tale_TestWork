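; RacePlayerState is the player state that replicates a racer's place, lap, checkpoint, name, final time, in-game and finished status.
; BeginPlay caches the local RacePlayerController, retrying once after a short delay if player controller 0 is not yet valid.
; On clients, RepNotifies call that controller's update events for player info, lap or checkpoint, while the FinalTime notify is empty.
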(event EventBeginPlay
  (bind _returnvalue (Game|GetPlayerController 0))
  (Utilities|IsValid _returnvalue :!label _label
    (:Is%20Valid
      (bind _asrace_player_controller (Utilities|Casting|CastToRacePlayerController _returnvalue))
      (Variables|Default|SetThisPlayerController _asrace_player_controller))
    (:Is%20Not%20Valid
      (if (not (Variables|Default|GetDelayed))
        (Variables|Default|SetDelayed true)
        (Utilities|FlowControl|Delay 0.2)
        (goto _label)))))

(fn ConstructionScript)

(fn OnRepCurrentPlace
  (bind _thisplayercontroller (Variables|Default|GetThisPlayerController))
  (Networking|SwitchHasAuthority
    (:Remote
      (Utilities|IsValid _thisplayercontroller
        (:Is%20Valid
          (Default|EUpdatePlayersInfo _thisplayercontroller))))))

(fn OnRepFinalTime)

(fn OnRepCurrentLap
  (Networking|SwitchHasAuthority
    (:Remote
      (Default|EUpdateCurrentLap (Variables|Default|GetThisPlayerController)))))

(fn OnRepLastCheckPointIndex
  (Networking|SwitchHasAuthority
    (:Remote
      (Default|EUpdatePlayerLastCheckPoint (Variables|Default|GetThisPlayerController)))))

(fn OnRepPlayerRaceName
  (Networking|SwitchHasAuthority
    (:Remote
      (Default|EUpdatePlayersInfo (Variables|Default|GetThisPlayerController)))))

(fn OnRepinGame
  (Networking|SwitchHasAuthority
    (:Remote
      (Default|EUpdatePlayersInfo (Variables|Default|GetThisPlayerController)))))

(fn OnRepFinished
  (Networking|SwitchHasAuthority
    (:Remote
      (Default|EUpdatePlayersInfo (Variables|Default|GetThisPlayerController)))))