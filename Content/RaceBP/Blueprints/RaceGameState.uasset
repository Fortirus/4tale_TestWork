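; RaceGameState is a game state Blueprint that holds the checkpoint count and lap count for a race.
; On BeginPlay, only with authority, it casts and caches the RaceGameMode.
; It then copies the number of level checkpoints from that mode's CheckPointSystem and the lap total from its RaceSettings.
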(event EventBeginPlay
  (Networking|SwitchHasAuthority
    (:Authority
      (bind _asrace_game_mode (Utilities|Casting|CastToRaceGameMode (Game|GetGameMode)))
      (bind _output_get (Variables|Default|SetThisRaceGameMode _asrace_game_mode))
      (Variables|RaceInfo|SetCheckPointsAmount (Utilities|Array|Length (Variables|/Game/Level/BP_CheckPointSystem.BP_CheckPointSystem_C|GetLevelCheckPoints (Variables|/Game/RaceBP/Blueprints/RaceGameMode.RaceGameMode_C|GetCheckPointSystem _output_get))))
      (Variables|RaceInfo|SetLapsAmount (Variables|/Game/Level/BP_RaceSettings.BP_RaceSettings_C|GetLapsAmount (Variables|/Game/RaceBP/Blueprints/RaceGameMode.RaceGameMode_C|GetRaceSettings _output_get))))))

(fn ConstructionScript)