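; Race game mode that registers players, spawns their cars at tag-ordered PlayerStarts and tracks laps, checkpoints and finishes.
; Player state lists are mirrored into RaceGameState, and finishers move to its results list.
; A Delay-throttled Tick measures next-checkpoint distances, then ranks racers with swap-sort passes by lap, checkpoint and distance, offset by finished count.
; Respawn teleports a car to its last checkpoint and clears its velocity.
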(event Custom|eSpawn%20Player
  (params (PlayerIndex :type Integer) (Controller :type Race%20Player%20Controller%20Object%20Reference))
  (bind _playersstates (Variables|Network|GetPlayersStates))
  (bind _output (Utilities|Array|Get(acopy) _playersstates PlayerIndex))
  (bind _output_get (Variables|Default|SetCurrentPlayerController Controller))
  (bind _returnvalue (Game|SpawnActorfromClass "/Game/RaceBP/RaceCar/BP_ArcadeCar.BP_ArcadeCar_C" (Transformation|GetActorTransform (Utilities|Array|Get(acopy) (Variables|Network|GetPlayersStarts) PlayerIndex)) "Undefined" _output_get 0))
  (Utilities|Array|Add (Variables|Network|GetPlayersCars) _returnvalue)
  (Pawn|Possess (Variables|Default|GetCurrentPlayerController) _returnvalue)
  (Variables|/Game/RaceBP/Blueprints/RacePlayerState.RacePlayerState_C|SetInGame _output true)
  (CallFunction|AddPlayerState _output true)
  (Default|EPawnSpawned (Variables|Default|GetCurrentPlayerController))
  (CallFunction|EChangePlayerLastCheckPoint 0 (Variables|Default|GetCurrentPlayerController)))

(event Custom|ePlayerGoNextLap
  (params (Controller :type Race%20Player%20Controller%20Object%20Reference))
  (CallFunction|SetPlayerLapEnd Controller))

(event Custom|eChangePlayerLastCheckPoint
  (params (CheckPointIndex :type Integer) (Controller :type Race%20Player%20Controller%20Object%20Reference))
  (bind _checkpointsystem (Variables|Default|GetCheckPointSystem))
  (Variables|/Game/RaceBP/Blueprints/RacePlayerController.RacePlayerController_C|SetNextCheckPoint Controller (Utilities|Array|Get(acopy) (Variables|/Game/Level/BP_CheckPointSystem.BP_CheckPointSystem_C|GetLevelCheckPoints _checkpointsystem) (Default|GetNextCheckPointIndex _checkpointsystem CheckPointIndex)))
  (Variables|/Game/RaceBP/Blueprints/RacePlayerState.RacePlayerState_C|SetLastCheckPointIndex (Variables|/Game/RaceBP/Blueprints/RacePlayerController.RacePlayerController_C|GetThisRacePlayerState Controller) CheckPointIndex))

(event Custom|eRespawnAtLastCheckPoint
  (params (PlayerCar :type BP%20Arcade%20Car%20Object%20Reference))
  (bind _output (CallFunction|GetPlayerLastCheckPoint PlayerCar))
  (bind _mesh (Variables|/Script/PhysXVehicles.WheeledVehicle|GetMesh PlayerCar))
  (Transformation|Teleport PlayerCar (Transformation|GetActorLocation _output) (Transformation|GetActorRotation _output))
  (Class|PrimitiveComponent|SetAllPhysicsLinearVelocity _mesh "0, 0, 0" false)
  (Class|PrimitiveComponent|SetAllPhysicsAngularVelocityinDegrees _mesh (Math|Vector|MakeVector 0.0 0.0 0.0) false))

(event EventBeginPlay
  (Utilities|FlowControl|Sequence
    (:then_0
      (bind _returnvalue (Actor|GetActorOfClass "/Game/Level/BP_CheckPointSystem.BP_CheckPointSystem_C"))
      (Variables|Default|SetCheckPointSystem _returnvalue)
      (bind _returnvalue_2 (Actor|GetActorOfClass "/Game/Level/BP_RaceSettings.BP_RaceSettings_C"))
      (Variables|Default|SetRaceSettings _returnvalue_2))
    (:then_1
      (bind _asrace_game_state (Utilities|Casting|CastToRaceGameState (Game|GetGameState))
        (:then
          (Variables|Default|SetThisRaceGameState _asrace_game_state))
        (:CastFailed
          _))
      (bind _outactors (Actor|GetAllActorsOfClass "/Script/Engine.PlayerStart"))
      (for _array_element _outactors
        (Utilities|Array|Insert (Variables|Network|GetPlayersStarts) _array_element (CallFunction|PlayerStartTagtoInt _array_element))))))

(event EventPostLogin
  (params (NewPlayer :type Player%20Controller%20Object%20Reference))
  (bind _asrace_player_controller (Utilities|Casting|CastToRacePlayerController NewPlayer))
  (Utilities|Array|Add (Variables|Network|GetPlayersControllers) _asrace_player_controller)
  (bind _asrace_player_state (Utilities|Casting|CastToRacePlayerState (Variables|/Script/Engine.Controller|GetPlayerState _asrace_player_controller)))
  (bind _playerstateindex (CallFunction|AddPlayerState _asrace_player_state false))
  (bind _output_get (Variables|/Game/RaceBP/Blueprints/RacePlayerState.RacePlayerState_C|SetPlayerIndex _asrace_player_state _playerstateindex))
  (Variables|/Game/RaceBP/Blueprints/RacePlayerState.RacePlayerState_C|SetCurrentPlace _asrace_player_state _output_get))

(event EventTick
  (params (DeltaSeconds :type Float%20%28single-precision%29))
  (Utilities|FlowControl|Delay 0.5)
  (for (_array_element _array_index) (Variables|Network|GetPlayersControllers)
    ;[1 1 1] Calculation of the distance to the next Check Point
    (bind _playerstate (Utilities|IsPlayerinGame _array_index)
      (:Yes
        (Variables|/Game/RaceBP/Blueprints/RacePlayerState.RacePlayerState_C|SetNextCheckPoint_Distance _playerstate (Math|Float|Truncate (Math|Vector|Distance(Vector) (Transformation|GetActorLocation (Variables|/Game/RaceBP/Blueprints/RacePlayerController.RacePlayerController_C|GetNextCheckPoint _array_element)) (Transformation|GetActorLocation (Pawn|GetControlledPawn _array_element))))))))
  (CallFunction|CalculatePlayerPlases))

(fn ConstructionScript)

(fn PlayerStartTagtoInt
  (params (PlayerStart :type Player%20Start%20Object%20Reference))
  (return (Math|Conversions|ToInteger(Byte) (Utilities|String|ToString(Name) (Variables|/Script/Engine.PlayerStart|GetPlayerStartTag PlayerStart)))))

(fn CalculatePlayerPlases
  (bind _playersstatesingame (Variables|Network|GetPlayersStatesInGame))
  (bind _returnvalue (Utilities|Array|LastIndex _playersstatesingame))
  (if (> _returnvalue 0) ; Two or more
    (LocalVariables|SetLastIndex _returnvalue)
    (bind _output_get (LocalVariables|SetPlayerStatesByPlace _playersstatesingame))
    ;[1 1 1] Sort by Values
    (for (_array_element _array_index) _output_get :!label _label
      (for _index (range _array_index (LocalVariables|GetLastIndex))
        (switch Utilities|FlowControl|Switch|SwitchonENUM_RaceComparisonType (LocalVariables|GetCurComparisonType)
          (:NewEnumerator0
            (if (> (Variables|/Game/RaceBP/Blueprints/RacePlayerState.RacePlayerState_C|GetCurrentLap (Utilities|Array|Get(acopy) (LocalVariables|GetPlayerStatesByPlace) _index)) (Variables|/Game/RaceBP/Blueprints/RacePlayerState.RacePlayerState_C|GetCurrentLap _array_element))
              (Utilities|Array|Swap (LocalVariables|GetPlayerStatesByPlace) _index _array_index :!label _label_2)))
          (:NewEnumerator1
            (if (and (== (Variables|/Game/RaceBP/Blueprints/RacePlayerState.RacePlayerState_C|GetCurrentLap (Utilities|Array|Get(acopy) (LocalVariables|GetPlayerStatesByPlace) _index)) (Variables|/Game/RaceBP/Blueprints/RacePlayerState.RacePlayerState_C|GetCurrentLap _array_element)) (> (Variables|/Game/RaceBP/Blueprints/RacePlayerState.RacePlayerState_C|GetLastCheckPointIndex (Utilities|Array|Get(acopy) (LocalVariables|GetPlayerStatesByPlace) _index)) (Variables|/Game/RaceBP/Blueprints/RacePlayerState.RacePlayerState_C|GetLastCheckPointIndex _array_element)))
              (goto _label_2)))
          (:NewEnumerator2
            (if (and (== (Variables|/Game/RaceBP/Blueprints/RacePlayerState.RacePlayerState_C|GetLastCheckPointIndex (Utilities|Array|Get(acopy) (LocalVariables|GetPlayerStatesByPlace) _index)) (Variables|/Game/RaceBP/Blueprints/RacePlayerState.RacePlayerState_C|GetLastCheckPointIndex _array_element)) (< (Variables|/Game/RaceBP/Blueprints/RacePlayerState.RacePlayerState_C|GetNextCheckPoint_Distance (Utilities|Array|Get(acopy) (LocalVariables|GetPlayerStatesByPlace) _index)) (Variables|/Game/RaceBP/Blueprints/RacePlayerState.RacePlayerState_C|GetNextCheckPoint_Distance _array_element)))
              (goto _label_2))))))
    (switch Utilities|FlowControl|Switch|SwitchonENUM_RaceComparisonType (LocalVariables|GetCurComparisonType)
      (:NewEnumerator0
        (LocalVariables|SetCurComparisonType "NewEnumerator1")
        (goto _label))
      (:NewEnumerator1
        (LocalVariables|SetCurComparisonType "NewEnumerator2")
        (goto _label))
      (:NewEnumerator2
        ;[1 1 1] Set new Place if needed
        (for (_array_element_2 _array_index_2) (LocalVariables|GetPlayerStatesByPlace)
          (if (!= (Variables|/Game/RaceBP/Blueprints/RacePlayerState.RacePlayerState_C|GetCurrentPlace _array_element_2) _array_index_2)
            (Variables|/Game/RaceBP/Blueprints/RacePlayerState.RacePlayerState_C|SetCurrentPlace _array_element_2 (+ _array_index_2 (Variables|Default|GetFinishedPlayersAmount)))))))))

(fn GetPlayerLastCheckPoint
  (params (PlayerCar :type BP%20Arcade%20Car%20Object%20Reference))
  (return (Utilities|Array|Get(acopy) (Variables|/Game/Level/BP_CheckPointSystem.BP_CheckPointSystem_C|GetLevelCheckPoints (Variables|Default|GetCheckPointSystem)) (Variables|/Game/RaceBP/Blueprints/RacePlayerState.RacePlayerState_C|GetLastCheckPointIndex (Variables|/Game/RaceBP/RaceCar/BP_ArcadeCar.BP_ArcadeCar_C|GetThisRacePlayerState PlayerCar)))))

(fn SetPlayerLapEnd
  (params (TargetPlayerController :type Race%20Player%20Controller%20Object%20Reference))
  (bind _thisraceplayerstate (Variables|/Game/RaceBP/Blueprints/RacePlayerController.RacePlayerController_C|GetThisRacePlayerState TargetPlayerController))
  (bind _checkpointsystem (Variables|Default|GetCheckPointSystem))
  (bind _thisraceplayerstate_2 (Variables|/Game/RaceBP/Blueprints/RacePlayerController.RacePlayerController_C|GetThisRacePlayerState TargetPlayerController))
  (Variables|/Game/RaceBP/Blueprints/RacePlayerController.RacePlayerController_C|SetNextCheckPoint TargetPlayerController (Utilities|Array|Get(acopy) (Variables|/Game/Level/BP_CheckPointSystem.BP_CheckPointSystem_C|GetLevelCheckPoints _checkpointsystem) (Default|GetNextCheckPointIndex _checkpointsystem)))
  (Variables|/Game/RaceBP/Blueprints/RacePlayerState.RacePlayerState_C|SetLastCheckPointIndex _thisraceplayerstate 0)
  (if (== (Variables|/Game/RaceBP/Blueprints/RacePlayerState.RacePlayerState_C|GetCurrentLap _thisraceplayerstate) (Variables|/Game/RaceBP/Blueprints/RaceGameState.RaceGameState_C|GetLapsAmount (Variables|Default|GetThisRaceGameState)))
    ;[1 1 1] Ended the race
    (Default|ERaceEnd TargetPlayerController)
    (Utilities|Array|Add (Variables|/Game/RaceBP/Blueprints/RaceGameState.RaceGameState_C|GetResultPlayersPlaces (Variables|Default|GetThisRaceGameState)) _thisraceplayerstate_2)
    (CallFunction|RemovePlayerState _thisraceplayerstate_2 true)
    (Variables|/Game/RaceBP/Blueprints/RacePlayerState.RacePlayerState_C|SetFinished _thisraceplayerstate_2 true)
    (Math|Integer|IncrementInt (Variables|Default|GetFinishedPlayersAmount))
    (else
      (Variables|/Game/RaceBP/Blueprints/RacePlayerState.RacePlayerState_C|SetCurrentLap _thisraceplayerstate_2 (+ (Variables|/Game/RaceBP/Blueprints/RacePlayerState.RacePlayerState_C|GetCurrentLap _thisraceplayerstate) 1)))))

(fn AddPlayerState
  (params (TargetPlayerState :type Race%20Player%20State%20Object%20Reference%20%28by%20ref%29) (InGameList :type Boolean))
  (bind _thisracegamestate (Variables|Default|GetThisRaceGameState))
  (if InGameList
    (Utilities|Array|AddUnique (Variables|Network|GetPlayersStatesInGame) TargetPlayerState)
    (bind _returnvalue (Utilities|Array|AddUnique (Variables|/Game/RaceBP/Blueprints/RaceGameState.RaceGameState_C|GetPlayersStatesInGame _thisracegamestate) TargetPlayerState))
    (return _returnvalue)
    (else
      (Utilities|Array|AddUnique (Variables|Network|GetPlayersStates) TargetPlayerState)
      (bind _returnvalue_2 (Utilities|Array|AddUnique (Variables|/Game/RaceBP/Blueprints/RaceGameState.RaceGameState_C|GetPlayersStates _thisracegamestate) TargetPlayerState))
      (return _returnvalue_2))))

(fn RemovePlayerState
  (params (TargetPlayerState :type Race%20Player%20State%20Object%20Reference%20%28by%20ref%29) (InGameList :type Boolean))
  (bind _thisracegamestate (Variables|Default|GetThisRaceGameState))
  (if InGameList
    (Utilities|Array|RemoveItem (Variables|Network|GetPlayersStatesInGame) TargetPlayerState)
    (Utilities|Array|RemoveItem (Variables|/Game/RaceBP/Blueprints/RaceGameState.RaceGameState_C|GetPlayersStatesInGame _thisracegamestate) TargetPlayerState)
    (else
      (Utilities|Array|RemoveItem (Variables|Network|GetPlayersStates) TargetPlayerState)
      (Utilities|Array|RemoveItem (Variables|/Game/RaceBP/Blueprints/RaceGameState.RaceGameState_C|GetPlayersStates _thisracegamestate) TargetPlayerState))))