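; Player controller for a networked racing game, bridging each player's UI with the game mode and player state.
; The local client shows a login screen, whose name and player index go through the server login event to the game mode for pawn spawning.
; After spawning, it swaps to the race HUD and forwards lap, checkpoint, player board and race-end updates.
; Inputs request respawn at the last checkpoint and toggle checkpoint debug meshes.
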(event Custom|eLogin
  (params (PlayerIndex :type Integer) (PlayerName :type String))
  (CallFunction|ELoginServer PlayerIndex PlayerName))

(event Custom|eLogin%20Server
  (params (PlayerIndex :type Integer) (PlayerName :type String))
  (Variables|/Game/RaceBP/Blueprints/RacePlayerState.RacePlayerState_C|SetPlayerRaceName (Variables|Default|GetThisRacePlayerState) PlayerName)
  (Default|ESpawnPlayer (Variables|Default|GetThisGameMode) PlayerIndex self))

(event Custom|ePawnSpawned
  (Widget|RemovefromParent (Variables|Default|GetLoginScreen))
  (Utilities|FlowControl|Delay 0.1) ; Delay for Car actor to spawn
  (bind _returnvalue (UserInterface|CreateWidget "/Game/RaceBP/Blueprints/WBP_PlayerUI.WBP_PlayerUI_C" self))
  (bind _output_get (Variables|Default|SetMainPlayerUI _returnvalue))
  (Variables|Default|SetCurrentMainWidget _output_get)
  (UserInterface|Viewport|AddtoViewport _output_get 0)
  (CallFunction|ChageInputModeto false) ; Change to Game Only
  (CallFunction|EUpdateCurrentLap)
  (CallFunction|EUpdatePlayerLastCheckPoint))

(event Custom|eCallRespawn
  (Default|ERespawnatLastCheckPoint (Variables|Default|GetThisGameMode) (.AsBP%20Arcade%20Car (Utilities|Casting|CastToBP_ArcadeCar (Pawn|GetControlledPawn)))))

(event Custom|eUpdatePlayersInfo
  ;[1 1 1] Network info and UI update on client
  (Utilities|SwitchMainUIValid
    (:Is%20Valid
      (Default|EUpdatePlayersInfoBoard (Variables|Default|GetMainPlayerUI)))))

(event Custom|eUpdatePlayerLastCheckPoint
  ;[1 1 1] Network info and UI update on client
  (Utilities|SwitchMainUIValid
    (:Is%20Valid
      (Default|EUpdateCheckPointsLeft (Variables|Default|GetMainPlayerUI)))))

(event Custom|eUpdateCurrentLap
  (bind _mainplayerui (Variables|Default|GetMainPlayerUI))
  ;[1 1 1] Network info and UI update on client
  (Utilities|SwitchMainUIValid
    (:Is%20Valid
      (Default|EUpdateLap _mainplayerui)
      (Default|EUpdateCheckPointsLeft _mainplayerui))))

(event Custom|eRaceEnd
  (Utilities|FlowControl|Delay 0.2)
  (Default|ERaceEnd (Variables|Default|GetMainPlayerUI))
  (Input|DisableInput (Pawn|GetControlledPawn) self))

(event EventBeginPlay
  (bind _self self)
  (if (Pawn|IsLocalController)
    ;[1 1 1] For Client
    (Utilities|FlowControl|Sequence
      (:then_0
        ;[1 1 1] Widgets and UI
        (Development|ExecuteConsoleCommand "t.maxfps 60" _self)
        (bind _returnvalue (UserInterface|CreateWidget "/Game/RaceBP/Blueprints/WBP_LoginScreen.WBP_LoginScreen_C" _self))
        (bind _output_get (Variables|Default|SetLoginScreen _returnvalue))
        (Variables|Default|SetCurrentMainWidget _output_get)
        (UserInterface|Viewport|AddtoViewport _output_get 0)
        (CallFunction|ChageInputModeto true) ; Start with UI input to enter player name
      )
      (:then_1
        ;[1 1 1] Network
        (bind _asrace_game_state (Utilities|Casting|CastToRaceGameState (Game|GetGameState)))
        (Variables|Default|SetThisRaceGameState _asrace_game_state)
        (Utilities|FlowControl|Delay 0.5) ; Wait for PlayerState
        (bind _asrace_player_state (Utilities|Casting|CastToRacePlayerState (Variables|GetPlayerState)))
        (Variables|Default|SetThisRacePlayerState _asrace_player_state))
      (:then_2
        (bind _returnvalue_2 (Actor|GetActorOfClass "/Game/Level/BP_CheckPointSystem.BP_CheckPointSystem_C"))
        (bind _output_get_2 (Variables|Default|SetCheckPointSystem _returnvalue_2))
        (Variables|Default|SetTestMode (Variables|/Game/Level/BP_CheckPoint.BP_CheckPoint_C|GetUseMesh (Utilities|Array|Get(acopy) (Variables|/Game/Level/BP_CheckPointSystem.BP_CheckPointSystem_C|GetLevelCheckPoints _output_get_2))))))
    (else
      ;[1 1 1] For Server
      (bind _asrace_game_mode (Utilities|Casting|CastToRaceGameMode (Game|GetGameMode)))
      (Variables|Default|SetThisGameMode _asrace_game_mode)
      (bind _asrace_player_state_2 (Utilities|Casting|CastToRacePlayerState (Variables|GetPlayerState)))
      (Variables|Default|SetThisRacePlayerState _asrace_player_state_2))))

(event Input|ActionEvents|InputActionRespawn
  (params (Key :type Key%20Structure :default "None"))
  (:Pressed
    (CallFunction|ECallRespawn)))

(event Input|ActionEvents|InputActionSwitchTestMode
  (params (Key :type Key%20Structure :default "None"))
  (bind _checkpointsystem (Variables|Default|GetCheckPointSystem))
  (:Pressed
    (bind _output_get (Variables|Default|SetTestMode (not (Variables|Default|GetTestMode))))
    (Default|SetChPMeshVis _checkpointsystem _output_get)
    (Default|SetOoBMeshVis _checkpointsystem _output_get)))

(fn ConstructionScript)

(fn ChageInputModeto
  (params (To%20UI%20only :type Boolean))
  (bind _self self)
  (if To%20UI%20only
    (Input|SetInputModeUIOnly _self (Variables|Default|GetCurrentMainWidget) "DoNotLock")
    (Variables|Default|SetbShowMouseCursor true)
    (else
      (Input|SetInputModeGameOnly _self)
      (Variables|Default|SetbShowMouseCursor false))))