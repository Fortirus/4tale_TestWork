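; Track actor that places instanced copies of a chosen mesh along a spline.
; The construction script sets the mesh and optional material, derives spacing from the mesh's X bound plus an offset, then adds an instance at each step along the spline's length.
; Instances optionally rotate to follow the spline direction.
; Collision type is reapplied on BeginPlay because the construction script setting does not stick.
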(event EventBeginPlay
  (CallFunction|UpdateMeshCollision) ; For some reason this parameter is not updated in the Construction Script
)

(fn ConstructionScript
  (bind _oversetobjectmaterial (Variables|Default|GetOversetObjectMaterial))
  (bind _roadpartinststaticmesh (Variables|Default|GetRoadPartInstStaticMesh))
  (bind _roadpartmesh (Variables|Default|GetRoadPartMesh))
  (bind _returnvalue (StaticMesh|GetBoundingBox _roadpartmesh))
  (Utilities|FlowControl|Sequence
    (:then_0
      (Components|StaticMesh|SetStaticMesh _roadpartinststaticmesh _roadpartmesh)
      (Utilities|IsValid _oversetobjectmaterial
        (:Is%20Valid
          (Rendering|Material|SetMaterial _roadpartinststaticmesh 0 _oversetobjectmaterial))
        (:Is%20Not%20Valid
          _))
      (CallFunction|UpdateMeshCollision)
      (bind _output_get (LocalVariables|SetMeshBoundSize (- (.max _returnvalue) (.min _returnvalue))))
      (LocalVariables|SetSectionLenght (+ (.x _output_get) (Variables|Default|GetAlongOffset))))
    (:then_1
      (for _index (range 0 (.ReturnValue (Math|Float|Division(WholeandRemainder) (Spline|GetSplineLength (Variables|Default|GetRoadSpline)) (LocalVariables|GetSectionLenght))))
        (LocalVariables|SetDIstanceStart (* _index (LocalVariables|GetSectionLenght)))
        (LocalVariables|SetDIstanceEnd (+ (* _index (LocalVariables|GetSectionLenght)) (LocalVariables|GetSectionLenght)))
        (Components|InstancedStaticMesh|AddInstance (Variables|Default|GetRoadPartInstStaticMesh) (Math|Transform|MakeTransform (Spline|GetLocationatDistanceAlongSpline (Variables|Default|GetRoadSpline) (LocalVariables|GetDIstanceStart) "Local") (CallFunction|NewObjRotation (LocalVariables|GetDIstanceStart))))))))

(fn NewObjRotation
  (params (Target%20Distance :type Float%20%28single-precision%29))
  (if (Variables|Default|GetRotateAlong)
    (return (Math|Conversions|RotationFromXVector (Spline|GetDirectionatDistanceAlongSpline (Variables|Default|GetRoadSpline) Target%20Distance "Local")))
    (else
      (return "0, 0, 0"))))

(fn UpdateMeshCollision
  (Collision|SetCollisionEnabled (Variables|Default|GetRoadPartInstStaticMesh) (Variables|Default|GetCollisionType)))