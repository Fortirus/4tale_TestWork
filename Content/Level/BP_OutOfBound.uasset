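; BP_OutOfBound is a level volume that sends arcade cars back to their last checkpoint when they leave the track.
; On overlap, if enabled, it casts to BP_ArcadeCar, asks the RaceGameMode to respawn it and prints a message.
; Detection runs only on the server, as remote instances disable the box's collision.
; At BeginPlay an optional cube mesh is shown, scaled to match the box extent.
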(event OnComponentBeginOverlap(BoxCollision)
  (params (OverlappedComponent :type Primitive%20Component%20Object%20Reference) (OtherActor :type Actor%20Object%20Reference) (OtherComp :type Primitive%20Component%20Object%20Reference) (OtherBodyIndex :type Integer) (bFromSweep :type Boolean) (SweepResult :type Hit%20Result%20Structure%20%28by%20ref%29))
  (if (Variables|Default|GetEnabled)
    (bind _asbp_arcade_car (Utilities|Casting|CastToBP_ArcadeCar OtherActor))
    (bind _output_get (Variables|Default|SetCurCar _asbp_arcade_car))
    (Default|ERespawnatLastCheckPoint (Variables|Default|GetThisRaceGameMode) _output_get)
    (Development|PrintString (Utilities|String|Append "Player " (Utilities|GetDisplayName _output_get) "get out of bounds in " (Utilities|GetDisplayName self)))))

(event EventBeginPlay
  (CallFunction|UpdateMesh)
  (Networking|SwitchHasAuthority
    (:Authority
      (bind _asrace_game_mode (Utilities|Casting|CastToRaceGameMode (Game|GetGameMode)))
      (Variables|Default|SetThisRaceGameMode _asrace_game_mode))
    (:Remote
      (Collision|SetCollisionEnabled (Variables|Default|GetBoxCollision) "NoCollision"))))

(fn ConstructionScript)

(fn UpdateMesh
  (bind _meshcube (Variables|Default|GetMeshCube))
  (if (Variables|Default|GetUseMesh)
    (Transformation|SetRelativeScale3D _meshcube (/ (Variables|/Script/Engine.BoxComponent|GetBoxExtent (Variables|Default|GetBoxCollision)) 50))
    (Rendering|SetVisibility _meshcube true false)
    (else
      (Rendering|SetVisibility _meshcube false false))))