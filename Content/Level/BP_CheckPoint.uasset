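; BP_CheckPoint is a race checkpoint trigger volume that tracks each car's progress and lap completion.
; On the server it finds its order index in the game mode's checkpoint list; clients disable its collision.
; When an arcade car overlaps, it compares the player's last checkpoint index and tells the game mode to advance the checkpoint or start the next lap.
; An optional cube mesh is scaled at BeginPlay to show the box extent.
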(event OnComponentBeginOverlap(BoxCollision)
  (params (OverlappedComponent :type Primitive%20Component%20Object%20Reference) (OtherActor :type Actor%20Object%20Reference) (OtherComp :type Primitive%20Component%20Object%20Reference) (OtherBodyIndex :type Integer) (bFromSweep :type Boolean) (SweepResult :type Hit%20Result%20Structure%20%28by%20ref%29))
  (bind _thisracegamemode (Variables|Default|GetThisRaceGameMode))
  (bind _asbp_arcade_car (Utilities|Casting|CastToBP_ArcadeCar OtherActor))
  (Variables|Default|SetCurCar _asbp_arcade_car)
  (Utilities|IsValid (Variables|/Game/RaceBP/RaceCar/BP_ArcadeCar.BP_ArcadeCar_C|GetThisRacePlayerState _asbp_arcade_car)
    (:Is%20Valid
      (Utilities|CheckThisCPnext (Variables|/Game/RaceBP/Blueprints/RacePlayerState.RacePlayerState_C|GetLastCheckPointIndex (Variables|/Game/RaceBP/RaceCar/BP_ArcadeCar.BP_ArcadeCar_C|GetThisRacePlayerState _asbp_arcade_car))
        (:This%20is%20the%20Next%20one
          (Default|EChangePlayerLastCheckPoint _thisracegamemode (Variables|Default|GetCheckPointOrderIndex) (.AsRace%20Player%20Controller (Utilities|Casting|CastToRacePlayerController (Pawn|GetController (Variables|Default|GetCurCar))))))
        (:End%20of%20Lap
          (Default|EPlayerGoNextLap _thisracegamemode (.AsRace%20Player%20Controller (Utilities|Casting|CastToRacePlayerController (Pawn|GetController (Variables|Default|GetCurCar))))))))))

(event EventBeginPlay
  (CallFunction|UpdateMesh)
  (Networking|SwitchHasAuthority
    (:Authority
      (bind _asrace_game_mode (Utilities|Casting|CastToRaceGameMode (Game|GetGameMode)))
      (bind _output_get (Variables|Default|SetThisRaceGameMode _asrace_game_mode))
      (Variables|Default|SetCheckPointOrderIndex (Utilities|Array|FindItem (Variables|/Game/Level/BP_CheckPointSystem.BP_CheckPointSystem_C|GetLevelCheckPoints (Variables|/Game/RaceBP/Blueprints/RaceGameMode.RaceGameMode_C|GetCheckPointSystem _output_get)) self)))
    (:Remote
      (Collision|SetCollisionEnabled (Variables|Default|GetBoxCollision) "NoCollision"))))

(fn ConstructionScript)

(fn UpdateMesh
  (bind _meshcube (Variables|Default|GetMeshCube))
  (if (Variables|Default|GetUseMesh)
    (Transformation|SetRelativeScale3D _meshcube (/ (Variables|/Script/Engine.BoxComponent|GetBoxExtent (Variables|Default|GetBoxCollision)) 50))
    (Rendering|SetVisibility _meshcube true false)
    (else
      (Rendering|SetVisibility _meshcube false false))))