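; Level checkpoint manager that holds the ordered checkpoint list and resolves which checkpoint comes next.
; Next-checkpoint lookups by index or reference wrap from last to first, forming a loop; the construction script records the checkpoint count.
; On BeginPlay it gathers all BP_OutOfBound actors.
; Two helper functions toggle mesh visibility across all checkpoints or out-of-bounds actors.
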(event EventBeginPlay
  (bind _outactors (Actor|GetAllActorsOfClass "/Game/Level/BP_OutOfBound.BP_OutOfBound_C"))
  (Variables|Default|SetLevelOutOfBounds _outactors))

(fn ConstructionScript
  (Variables|Default|SetCheckPointsAmount (Utilities|Array|Length (Variables|Default|GetLevelCheckPoints))))

(fn GetNextCheckPointIndex
  (params (CurCheckPointIndex :type Integer))
  (if (>= CurCheckPointIndex (Utilities|Array|LastIndex (Variables|Default|GetLevelCheckPoints)))
    (return 0) ; LOOP
    (else
      (return (+ CurCheckPointIndex 1)))))

(fn GetNextCheckPoint
  (params (CurCheckPoint :type BP%20Check%20Point%20Object%20Reference))
  (bind _levelcheckpoints (Variables|Default|GetLevelCheckPoints))
  (bind _levelcheckpoints_2 (Variables|Default|GetLevelCheckPoints))
  (bind _returnvalue (Utilities|Array|FindItem _levelcheckpoints CurCheckPoint))
  (if (== _returnvalue -1)
    (return 0) ; if CheckPoint doesn't FOUND
    (elif (== _returnvalue (Utilities|Array|LastIndex _levelcheckpoints))
      (return (Utilities|Array|Get(acopy) _levelcheckpoints_2)) ; LOOP
      (else
        (return (Utilities|Array|Get(acopy) _levelcheckpoints_2 (+ _returnvalue 1)))))))

(fn SetChPMeshVis
  (params (SetTo :type Boolean))
  (for _array_element (Variables|Default|GetLevelCheckPoints)
    (Variables|/Game/Level/BP_CheckPoint.BP_CheckPoint_C|SetUseMesh _array_element SetTo)
    (Default|UpdateMesh _array_element)))

(fn SetOoBMeshVis
  (params (SetTo :type Boolean))
  (for _array_element (Variables|Default|GetLevelOutOfBounds)
    (Variables|/Game/Level/BP_OutOfBound.BP_OutOfBound_C|SetUseMesh _array_element SetTo)
    (Default|UpdateMesh _array_element)))